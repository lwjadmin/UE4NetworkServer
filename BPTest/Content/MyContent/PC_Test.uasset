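; Test PlayerController that passes each player's name from the local GameInstance to their PlayerState in a listen-server game.
; On possess it prints the pawn and calls ResClientProcess, commented as client-side, which reads DBPlayerInfo from GI_Test.
; That info goes to ReqUpdatePlayerInfo, commented as server-side, which sets the name on PS_Test.
; A separate function forwards a given name to RunServer, which sets it the same way.
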(event Custom|ResClientProcess
  ;[0 0 1] [Client] 모든 클라이언트는 서버로 자신의 GameInstance에 저장된 PlayerInfo를 전달!
  (bind _asgi_test (Utilities|Casting|CastToGI_Test (Game|GetGameInstance)))
  (CallFunction|ReqUpdatePlayerInfo (Variables|/Game/MyContent/GI_Test.GI_Test_C|GetDBPlayerInfo _asgi_test)))

(event Custom|ReqUpdatePlayerInfo
  (params (InPlayerInfo :type ST%20Player%20Info%20Structure))
  ;[1 0 0] [Server] 리슨서버는 각각의 PlayerState에 모든 클라이언트로부터 수신받은 PlayerInfo를 저장!
  (bind _asps_test (Utilities|Casting|CastToPS_Test (Variables|GetPlayerState)))
  (Default|SetPlayerName _asps_test (.PlayerName (Utilities|Struct|BreakST_PlayerInfo InPlayerInfo))))

(event Custom|RunServer
  (params (PlayerName :type String))
  (bind _asps_test (Utilities|Casting|CastToPS_Test (Variables|GetPlayerState)))
  (Default|SetPlayerName _asps_test PlayerName))

(event EventPossess
  (params (PossessedPawn :type Pawn%20Object%20Reference))
  ;[1 1 1] PlayerCharacter에 Possed되었을 때, ResClientProcess 호출!
  (Development|PrintString (Utilities|String|Append "PossedPawn : " (Utilities|GetDisplayName PossessedPawn)) true true "(R=0.993407,G=0.000000,B=1.000000,A=1.000000)" 6e+01)
  (CallFunction|ResClientProcess))

(fn ConstructionScript)

(fn FUCKYOU
  (params (PlayerName :type String))
  (CallFunction|RunServer PlayerName))